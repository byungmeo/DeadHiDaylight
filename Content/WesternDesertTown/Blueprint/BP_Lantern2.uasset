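; Lantern prop for the Western desert town with a flickering point light and a Niagara flame, configured entirely in the Construction Script.
; It creates dynamic instances of the light function and fire materials, randomizing blink offset and frequency per lantern.
; The fire material copies those values from the light's instance, so flame and light flicker share parameters.
; Exposed variables shape intensity, flame size and particle jitter, and EnableFlame toggles both components.
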(event EventBeginPlay)

(event Collision|EventActorBeginOverlap
  (params (OtherActor :type Actor%20Object%20Reference)))

(event EventTick
  (params (DeltaSeconds :type Float%20%28single-precision%29)))

(fn ConstructionScript
  (bind _niagara (Variables|Default|GetNiagara))
  (bind _blinking_min_level (Variables|Default|GetBlinking%20min%20level))
  (Utilities|FlowControl|Sequence
    (:then_0
      (bind _returnvalue (Rendering|Material|CreateDynamicMaterialInstance "/Game/WesternDesertTown/Material/MI_LightFunction.MI_LightFunction" "None" "None" :!class /Script/Engine.KismetMaterialLibrary))
      (Rendering|Components|Light|SetLightFunctionMaterial (Variables|Default|GetPointLight) _returnvalue)
      (Rendering|Material|SetScalarParameterValue _returnvalue "Random offset" (Math|Random|RandomFloatinRange 0.0 1e+02) :!class /Script/Engine.MaterialInstanceDynamic)
      (Utilities|FlowControl|Sequence
        (:then_0
          (Rendering|Material|SetScalarParameterValue _returnvalue "Blinking frequency" (Math|Float|Clamp(Float) (+ (Math|Random|RandomFloatinRange 0.9 1.1) (/ (- (Variables|Default|GetBlinking%20frequency) 1e+01) 1e+01)) 0.0 1.8e+02) :!class /Script/Engine.MaterialInstanceDynamic)
          (Utilities|FlowControl|Sequence
            (:then_0
              (Rendering|Material|SetScalarParameterValue _returnvalue "Blinking min level" _blinking_min_level :!class /Script/Engine.MaterialInstanceDynamic)
              (Rendering|Components|Light|SetIntensity (Variables|Default|GetPointLight) (Variables|Default|GetLight%20Intensity))
              (Rendering|SetVisibility (Variables|Default|GetPointLight) (Variables|Default|GetEnable%20flame) false))
            (:then_1
              (bind _returnvalue_2 (Rendering|Material|GetScalarParameterValue _returnvalue "Blinking frequency" :!class /Script/Engine.MaterialInstanceDynamic)))))
        (:then_1
          (bind _returnvalue_3 (Rendering|Material|GetScalarParameterValue _returnvalue "Random offset" :!class /Script/Engine.MaterialInstanceDynamic)))))
    (:then_1
      (bind _returnvalue_4 (Rendering|Material|CreateDynamicMaterialInstance "/Game/WesternDesertTown/Material/MI_Fire.MI_Fire" "None" "None" :!class /Script/Engine.KismetMaterialLibrary))
      (Class|NiagaraComponent|SetVariableMaterial _niagara "Material" _returnvalue_4)
      (Niagara|SetNiagaraVariable(Float) _niagara "Radius" (Math|Float|Lerp 0.0 0.3 (Variables|Default|GetParticle%20Jitter%20Intensity)))
      (Niagara|SetNiagaraVariable(Float) _niagara "Flame Width" (Variables|Default|GetFlame%20Width))
      (Niagara|SetNiagaraVariable(Float) _niagara "Flame Height" (Math|Float|Lerp 0.0 0.2 (Variables|Default|GetFlame%20Height)))
      (Rendering|Material|SetScalarParameterValue _returnvalue_4 "Random offset" _returnvalue_3 :!class /Script/Engine.MaterialInstanceDynamic)
      (Rendering|Material|SetScalarParameterValue _returnvalue_4 "Blinking frequency" _returnvalue_2 :!class /Script/Engine.MaterialInstanceDynamic)
      (Rendering|Material|SetScalarParameterValue _returnvalue_4 "Blinking min level" _blinking_min_level :!class /Script/Engine.MaterialInstanceDynamic)
      (Rendering|Material|SetScalarParameterValue _returnvalue_4 "Particle intensity" (Variables|Default|GetParticle%20intensity) :!class /Script/Engine.MaterialInstanceDynamic)
      (Rendering|SetVisibility (Variables|Default|GetNiagara) (Variables|Default|GetEnable%20flame) false))))